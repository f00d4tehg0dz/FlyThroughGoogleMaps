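; BP_WindComponent is a component that pushes its owner's physics-simulating static meshes with the wind from BP_DynamicVolumetricSky.
; On BeginPlay it collects those meshes and starts a looping timer at roughly 60 Hz.
; Each tick reads wind direction and speed from the first sky actor found, then applies a scaled force to every mesh as an acceleration change, so mass is ignored.
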(event Custom|MainTick
  (bind _outactors (Actor|GetAllActorsOfClass "/Game/DynamicVolumetricSky/Blueprints/BP_DynamicVolumetricSky.BP_DynamicVolumetricSky_C"))
  (for _array_element (Variables|Default|GetPhysicsMeshes)
    (Physics|AddForce _array_element (* (/ (* (Math|Vector|Normalize (Variables|/Game/DynamicVolumetricSky/Blueprints/BP_DynamicVolumetricSky.BP_DynamicVolumetricSky_C|GetWind%20Direction (Utilities|Array|Get(acopy) _outactors))) (* (Variables|/Game/DynamicVolumetricSky/Blueprints/BP_DynamicVolumetricSky.BP_DynamicVolumetricSky_C|GetWind%20Speed (Utilities|Array|Get(acopy) _outactors)) 36.0)) 0.016667) 1.293) "None" true)))

(event EventBeginPlay
  (for _array_element (Actor|GetComponentsByClass (Components|GetOwner) "/Script/Engine.StaticMeshComponent")
    (if (Physics|IsSimulatingPhysics _array_element "None")
      (Utilities|Array|Add (Variables|Default|GetPhysicsMeshes) _array_element)
      (Utilities|Time|SetTimerbyEvent (delegate Custom|MainTick) 0.016667 true))))